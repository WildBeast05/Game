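; Base enemy Blueprint, a sprite-based character that walks along world +X and takes damage until it dies.
; Tick feeds constant movement input, while AnyDamage subtracts from Health and triggers death only when it equals exactly zero.
; Death disables movement and capsule collision, flashes the sprite red via timed delays, and lays it over.
; The delayed DestroyActor chain is unconnected, so the actor is never destroyed here.
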(event `Death flash`
  (bind _sprite (`self.Sprite`))
  (`PaperFlipbookComponent.SetSpriteColor` _sprite (struct :`R` 1.0 :`A` 1.0))
  (`KismetSystemLibrary.Delay` 0.2)
  (`PaperFlipbookComponent.SetSpriteColor` _sprite (struct :`R` 1.0 :`G` 1.0 :`B` 1.0 :`A` 1.0))
  (`KismetSystemLibrary.Delay` 0.2)
  (`PaperFlipbookComponent.SetSpriteColor` _sprite (struct :`R` 1.0 :`A` 1.0))
  (`KismetSystemLibrary.Delay` 0.2)
  (`PaperFlipbookComponent.SetSpriteColor` _sprite (struct :`R` 1.0 :`G` 1.0 :`B` 1.0 :`A` 1.0)))

(event `self.ReceiveAnyDamage`
  (params (Damage :type "Float (single-precision)") (DamageType :type "DamageType Object Reference") (InstigatedBy :type "Controller Object Reference") (DamageCauser :type "Actor Object Reference"))
  (bind _output_get (set `self.Health` (- (`self.Health`) Damage)))
  (if (== _output_get 0.0)
    (set `self.isDead` true)
    (`ActorComponent.SetActive` (`self.CharacterMovement`) false false)
    (`PrimitiveComponent.SetCollisionEnabled` (`self.CapsuleComponent`) "NoCollision")
    (`self.Death flash`)
    (`SceneComponent.K2_SetRelativeLocationAndRotation` (`self.Sprite`) (0.0 0.0 -80.0) (struct :`Pitch` 90.0) false false)))

(event `self.ReceiveTick`
  (params (DeltaSeconds :type "Float (single-precision)"))
  (`KismetSystemLibrary.Delay` 0.0)
  (`/Engine/EditorBlueprintResources/StandardMacros.CompareFloat` (`KismetMathLibrary.GetTotalSeconds` (struct))
    (:`>`
      _)
    (:`==`
      _))
  (`self.AddMovementInput` (0.1 0.0 0.0)))

(fn `UserConstructionScript`)