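; An ammo pickup actor that gives the player three ammo and then destroys itself.
; Each Tick it polls PickUpArea for overlapping Player actors, adds ammo when one is player character 0, and sets Picked to trigger destruction.
; The debug print adds three again, so it shows more than the stored ammo.
; Logic to spin SpriteFlipbook around yaw exists but is disconnected and never runs.
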(event `self.ReceiveTick`
  (params (DeltaSeconds :type "Float (single-precision)"))
  (for _array_element (`PrimitiveComponent.GetOverlappingActors` (`self.PickUpArea`) "/Game/Reordered/Blueprints/Player/Player.Player_C")
    (if (== _array_element (`GameplayStatics.GetPlayerCharacter` 0))
      (bind _asplayer (cast `/Game/Reordered/Blueprints/Player/Player` (`GameplayStatics.GetPlayerCharacter` 0)))
      (bind _returnvalue (+ (`/Game/Reordered/Blueprints/Player/Player.Ammo` _asplayer) 3))
      (set `/Game/Reordered/Blueprints/Player/Player.Ammo` _returnvalue _asplayer)
      (set `self.Picked` true)
      (`KismetSystemLibrary.PrintString` (`KismetStringLibrary.Conv_IntToString` _returnvalue))))
  (if (`self.Picked`)
    (`self.K2_DestroyActor`)))

(fn `UserConstructionScript`)