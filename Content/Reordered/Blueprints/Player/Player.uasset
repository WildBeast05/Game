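; Player pawn for a side-scrolling game, with X-axis movement, interaction, shooting, health and death.
; Tick snaps control yaw and weapon offset to the direction of X velocity.
; Firing spends ammo, spawns a bullet and plays weapon and camera recoil timelines, with a DoOnce reset after a delay.
; Damage reveals the hidden HUD and restarts the level when health equals zero, while interaction messages overlapping actors through an interface.
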(event `EnhancedInput|/Game/Reordered/Blueprints/Input_Handling/Interact_F`
  (params (ActionValue :type Boolean) (ElapsedSeconds :type "Float (double-precision)") (TriggeredSeconds :type "Float (double-precision)") (InputAction :type "InputAction Object Reference" :default "/Game/Reordered/Blueprints/Input_Handling/Interact_F.Interact_F"))
  ;[1 1 1] Interact Code
  (:`Triggered`
    (for _array_element (`self.GetOverlappingActors` "/Script/Engine.Actor")
      (if (`KismetSystemLibrary.DoesImplementInterface` _array_element "/Game/Reordered/Blueprints/Interactable/Interact_Interface.Interact_Interface_C")
        (bind _sucsess (message `/Game/Reordered/Blueprints/Interactable/Interact_Interface.Interact` _array_element self))
        (if _sucsess
          (break))))))

(event `self.ReceiveAnyDamage`
  (params (Damage :type "Float (single-precision)") (DamageType :type "DamageType Object Reference") (InstigatedBy :type "Controller Object Reference") (DamageCauser :type "Actor Object Reference"))
  (bind _hud (`self.HUD`))
  (`|ExecutionSequence`
    (:`then_0`
      (bind _output_get (set `self.Health` (- (`self.Health`) Damage)))
      (if (== _output_get 0.0)
        (set `self.isDead` true)
        (`ActorComponent.SetActive` (`self.CharacterMovement`) false false)
        (`KismetSystemLibrary.Delay` 0.5)
        (`self.Restart Level`)))
    (:`then_1`
      (if (not (`Widget.IsVisible` _hud))
        (`Widget.SetVisibility` _hud "Visible")))))

(event `Key|LeftMouseButton`
  (params (Key :type "Key Structure"))
  (bind (_returnvalue_roll _returnvalue_pitch _returnvalue_yaw) (`KismetMathLibrary.BreakRotator` (`self.GetControlRotation`)))
  (bind _weapon (`self.Weapon`))
  (bind _camera (`self.Camera`))
  (bind (_relativelocation_x _relativelocation_y _relativelocation_z) (`KismetMathLibrary.BreakVector` (`SceneComponent.RelativeLocation` _weapon)))
  (bind (_relativelocation_x_2 _relativelocation_y_2 _relativelocation_z_2) (`KismetMathLibrary.BreakVector` (`SceneComponent.RelativeLocation` _camera)))
  (:`Pressed`
    (if (`self.hasGun`)
      (if (> (`self.Ammo`) 0)
        (`/Engine/EditorBlueprintResources/StandardMacros.DoOnce` false :!label _label
          (:`Completed`
            (set `self.Ammo` (- (`self.Ammo`) 1))
            (`GameplayStatics.PlaySound2D` "/Game/Reordered/Sounds/M1_Garand_Shot.M1_Garand_Shot" 1.0 1.0 0.0 null null)
            (`|SpawnActorFromClass` "/Game/Blueprints/Player/Bullet_BP.Bullet_BP_C" (`SceneComponent.K2_GetComponentToWorld` (`self.bullet_spawn`)) "Undefined" "MultiplyWithRoot" self null)
            (`/Engine/EditorBlueprintResources/StandardMacros.CompareFloat` _returnvalue_yaw
              (:`>`
                (set `self.rotation` 1.0))
              (:`==`
                (set `self.rotation` -1.0)))
            (`|ExecutionSequence`
              (:`then_0`
                (bind (_direction _newtrack_0) (`Timeline|Recoil_Camera` :!via `PlayFromStart`)
                  (:`Update`
                    (`SceneComponent.K2_SetRelativeLocation` _camera (`KismetMathLibrary.MakeVector` (`KismetMathLibrary.Lerp` 0.0 -2.0 _newtrack_0) (`KismetMathLibrary.Lerp` 0.0 (* 10.0 (`self.rotation`)) _newtrack_0) _relativelocation_z_2) false false))))
              (:`then_1`
                (bind (_direction_2 _newtrack_0_2) (`Timeline|Recoil` :!via `PlayFromStart`)
                  (:`Update`
                    (`SceneComponent.K2_SetRelativeLocation` _weapon (`KismetMathLibrary.MakeVector` (`KismetMathLibrary.Lerp` -12.5 -14.5 _newtrack_0_2) _relativelocation_y _relativelocation_z) false false)
                    (`KismetSystemLibrary.Delay` 1.0)
                    (goto _label :!via `Reset`)))))))))))

(event `self.ReceiveTick`
  (params (DeltaSeconds :type "Float (single-precision)"))
  (`self.Rotate Player`))

(event `EnhancedInput|/Game/Reordered/Blueprints/Input_Handling/Movement_On_X_Axis`
  (params (ActionValue :type "Float (double-precision)") (ElapsedSeconds :type "Float (double-precision)") (TriggeredSeconds :type "Float (double-precision)") (InputAction :type "InputAction Object Reference" :default "/Game/Reordered/Blueprints/Input_Handling/Movement_On_X_Axis.Movement_On_X_Axis"))
  (:`Triggered`
    (`self.AddMovementInput` (1.0 0.0 0.0) ActionValue)))

(event `self.ReceiveBeginPlay`
  (bind _asplayer_controller (cast `PlayerController` (`GameplayStatics.GetPlayerController` 0)))
  (bind _returnvalue (pcsubsystem `EnhancedInputLocalPlayerSubsystem` _asplayer_controller))
  (`/Engine/EditorBlueprintResources/StandardMacros.IsValid` _returnvalue
    (:`Is Valid`
      (`EnhancedInputSubsystemInterface.AddMappingContext` _returnvalue "/Game/Reordered/Blueprints/Input_Handling/Main_Input_Mapping_Context.Main_Input_Mapping_Context" 0 (struct))
      (bind _returnvalue_2 (`|CreateWidget` "/Game/Reordered/Blueprints/Player/HUD.HUD_C"))
      (bind _output_get (set `self.HUD` _returnvalue_2))
      (`UserWidget.AddToViewport` _output_get 0)
      (`Widget.SetVisibility` _output_get "Hidden"))))

(fn `Restart Level`
  (bind _returnvalue (`GameplayStatics.GetCurrentLevelName` true))
  (`GameplayStatics.OpenLevel` (`KismetStringLibrary.Conv_StringToName` _returnvalue)))

(fn `Rotate Player`
  (bind _returnvalue (`self.GetController`))
  (bind _weapon (`self.Weapon`))
  (bind _velocity_x (`KismetMathLibrary.BreakVector` (`MovementComponent.Velocity` (`self.CharacterMovement`))))
  (bind (_relativelocation_x _relativelocation_y _relativelocation_z) (`KismetMathLibrary.BreakVector` (`SceneComponent.RelativeLocation` _weapon)))
  (`/Engine/EditorBlueprintResources/StandardMacros.CompareFloat` _velocity_x
    (:`>`
      (`Controller.SetControlRotation` _returnvalue (`KismetMathLibrary.MakeRotator` 0.0))
      (`SceneComponent.K2_SetRelativeLocation` _weapon (`KismetMathLibrary.MakeVector` _relativelocation_x 0.01 _relativelocation_z) false false))
    (:`<`
      (`Controller.SetControlRotation` _returnvalue (`KismetMathLibrary.MakeRotator` 0.0 0.0 180.0))
      (`SceneComponent.K2_SetRelativeLocation` _weapon (`KismetMathLibrary.MakeVector` _relativelocation_x -0.01 _relativelocation_z) false false))))

(fn `UserConstructionScript`)