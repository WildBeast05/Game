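; Interactable flipbook door that takes the player to the hard-coded Outside_House_Weaponless level.
; Overlapping its box as the player shows an interact prompt widget, removed on leaving or opening.
; Interact runs a one-shot open: camera fade to black, sound, and a timeline that swings and darkens the flipbook before loading the level.
; The close branch reverses the timeline, but the IsOpen toggle and DoOnce reset are unconnected.
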(event `Open Door`
  (`/Engine/EditorBlueprintResources/StandardMacros.DoOnce` false
    (:`Completed`
      (`PlayerCameraManager.StartCameraFade` :`self` (`GameplayStatics.GetPlayerCameraManager` 0) :`ToAlpha` 1.0 :`Duration` 1.0 :`bHoldWhenFinished` true)
      (`GameplayStatics.PlaySound2D` "/Game/Reordered/Sounds/Door_Open.Door_Open" 1.0 1.0 0.0 null null)
      (`Widget.RemoveFromParent` (`self.InteractPrompt`))
      (bind (_direction _door_track) (`Timeline|Open Door T` :!label _label)
        (:`Update`
          (`SceneComponent.K2_SetRelativeRotation` (`self.PaperFlipbook`) (`KismetMathLibrary.MakeRotator` 0.0 0.0 (`KismetMathLibrary.Lerp` 0.0 90.0 _door_track)) false false)
          (`PaperFlipbookComponent.SetSpriteColor` (`self.PaperFlipbook`) (`KismetMathLibrary.LinearColorLerpUsingHSV` (struct :`R` 1.0 :`G` 1.0 :`B` 1.0 :`A` 1.0) (struct :`A` 1.0) _door_track)))
        (:`Finished`
          (`KismetSystemLibrary.Delay` 0.0)
          (`GameplayStatics.OpenLevel` "Outside_House_Weaponless"))))))

(event `Close Door`
  (goto _label :!via `Reverse`))

(event `self.ReceiveBeginPlay`
  (bind _returnvalue (`|CreateWidget` "/Game/Reordered/UI/Prompt_Interact.Prompt_Interact_C"))
  (set `self.InteractPrompt` _returnvalue))

(event `self.Box.OnComponentBeginOverlap`
  (params (OverlappedComponent :type "PrimitiveComponent Object Reference") (OtherActor :type "Actor Object Reference") (OtherComp :type "PrimitiveComponent Object Reference") (OtherBodyIndex :type Integer) (bFromSweep :type Boolean) (SweepResult :type "HitResult Structure (by ref)"))
  (if (== OtherActor (`GameplayStatics.GetPlayerCharacter` 0))
    (`UserWidget.AddToViewport` (`self.InteractPrompt`) 0)))

(event `self.Box.OnComponentEndOverlap`
  (params (OverlappedComponent :type "PrimitiveComponent Object Reference") (OtherActor :type "Actor Object Reference") (OtherComp :type "PrimitiveComponent Object Reference") (OtherBodyIndex :type Integer))
  (if (== (`GameplayStatics.GetPlayerCharacter` 0) OtherActor)
    (`Widget.RemoveFromParent` (`self.InteractPrompt`))))

(fn `Interact`
  (params (Interactor :type "Character Object Reference"))
  (returns (Sucsess :type Boolean))
  (if (not (`self.isOpen`))
    (`TimelineComponent.SetPlayRate` (`self.Open Door T`) (/ 1.0 (`self.TimeToOpen`)))
    (`self.Open Door`)
    (else
      (`TimelineComponent.SetPlayRate` (`self.Open Door T`) (/ 1.0 (`self.TimeToOpen`)))
      (`self.Close Door`)))
  (return true))

(fn `UserConstructionScript`)