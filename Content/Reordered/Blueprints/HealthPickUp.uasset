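; Health pickup actor that spins and grants the player one point of health, then destroys itself.
; Each Tick yaws the flipbook sprite and polls PickUpArea's overlapping actors for the player pawn to set a Picked flag.
; While Picked, it heals only if Health is below five.
; Picked never resets, so a pickup touched at full health persists and applies once health drops, even from afar.
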(event `self.ReceiveTick`
  (params (DeltaSeconds :type "Float (single-precision)"))
  (bind _sprite_flipbook (`self.Sprite_Flipbook`))
  (bind (_returnvalue_roll _returnvalue_pitch _returnvalue_yaw) (`KismetMathLibrary.BreakRotator` (`SceneComponent.K2_GetComponentRotation` _sprite_flipbook)))
  (`|ExecutionSequence`
    (:`then_0`
      (`SceneComponent.K2_SetWorldRotation` _sprite_flipbook (`KismetMathLibrary.MakeRotator` _returnvalue_roll _returnvalue_pitch (+ _returnvalue_yaw 3.0)) false false))
    (:`then_1`
      (for _array_element (`PrimitiveComponent.GetOverlappingActors` (`self.PickUpArea`) "/Game/Reordered/Blueprints/Player/Player.Player_C")
        (if (== _array_element (`GameplayStatics.GetPlayerPawn` 0))
          (set `self.Picked` true))))
    (:`then_2`
      (if (`self.Picked`)
        (bind _asplayer (cast `/Game/Reordered/Blueprints/Player/Player` (`GameplayStatics.GetPlayerCharacter` 0)))
        (bind _health (`/Game/Reordered/Blueprints/Player/Player.Health` _asplayer))
        (if (< _health 5.0)
          (set `/Game/Reordered/Blueprints/Player/Player.Health` (+ _health 1.0) _asplayer)
          (`self.K2_DestroyActor`))))))

(fn `UserConstructionScript`)