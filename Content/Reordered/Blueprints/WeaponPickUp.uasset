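; WeaponPickUp is an interactable weapon pickup that gives the player a gun.
; The PickUp overlap shows or removes an interact prompt widget, created at BeginPlay, as the player pawn enters or leaves.
; Interact fires Interacted, which casts the overlapping actor to Player, sets its weapon sprite and HasGun flag, destroys the pickup and reveals the HUD if hidden.
; Older HUD-creation logic remains unconnected.
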(event `Interacted`
  (bind _asplayer (cast `/Game/Reordered/Blueprints/Player/Player` (stale `self.PickUp.OnComponentBeginOverlap` OtherActor)))
  (`PaperSpriteComponent.SetSprite` (`/Game/Reordered/Blueprints/Player/Player.Weapon` _asplayer) "/Game/Reordered/Textures/Weapons/weapon_hand_Sprite.weapon_hand_Sprite")
  (set `/Game/Reordered/Blueprints/Player/Player.hasGun` true _asplayer)
  (`self.K2_DestroyActor`)
  (bind _hud (`/Game/Reordered/Blueprints/Player/Player.HUD` _asplayer))
  (if (not (`Widget.IsVisible` _hud))
    (`Widget.SetVisibility` _hud "Visible")))

(event `self.ReceiveBeginPlay`
  (bind _returnvalue (`|CreateWidget` "/Game/Reordered/UI/Prompt_Interact.Prompt_Interact_C"))
  (set `self.Interact_Prompt` _returnvalue))

(event `self.Box.OnComponentBeginOverlap`
  (params (OverlappedComponent :type "PrimitiveComponent Object Reference") (OtherActor :type "Actor Object Reference") (OtherComp :type "PrimitiveComponent Object Reference") (OtherBodyIndex :type Integer) (bFromSweep :type Boolean) (SweepResult :type "HitResult Structure (by ref)")))

(event `self.PickUp.OnComponentBeginOverlap`
  (params (OverlappedComponent :type "PrimitiveComponent Object Reference") (OtherActor :type "Actor Object Reference") (OtherComp :type "PrimitiveComponent Object Reference") (OtherBodyIndex :type Integer) (bFromSweep :type Boolean) (SweepResult :type "HitResult Structure (by ref)"))
  (if (== OtherActor (`GameplayStatics.GetPlayerPawn` 0))
    (`UserWidget.AddToViewport` (`self.Interact_Prompt`) 0)))

(event `self.PickUp.OnComponentEndOverlap`
  (params (OverlappedComponent :type "PrimitiveComponent Object Reference") (OtherActor :type "Actor Object Reference") (OtherComp :type "PrimitiveComponent Object Reference") (OtherBodyIndex :type Integer))
  (if (== OtherActor (`GameplayStatics.GetPlayerPawn` 0))
    (`Widget.RemoveFromParent` (`self.Interact_Prompt`))))

(fn `Interact`
  (params (Interactor :type "Character Object Reference"))
  (returns (Sucsess :type Boolean))
  (`self.Interacted`)
  (return true))

(fn `UserConstructionScript`)