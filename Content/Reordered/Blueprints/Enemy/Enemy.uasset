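; Enemy character Blueprint that walks steadily along world +X and can be killed by damage.
; BeginPlay activates character movement, and Tick feeds it a small constant movement input.
; AnyDamage subtracts from Health; only when Health equals exactly zero does it set IsDead, deactivate movement and disable capsule collision.
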(event `self.ReceiveAnyDamage`
  (params (Damage :type "Float (single-precision)") (DamageType :type "DamageType Object Reference") (InstigatedBy :type "Controller Object Reference") (DamageCauser :type "Actor Object Reference"))
  (bind _output_get (set `self.Health` (- (`self.Health`) Damage)))
  (if (== _output_get 0.0)
    (set `self.isDead` true)
    (`ActorComponent.SetActive` (`self.CharacterMovement`) false false)
    (`PrimitiveComponent.SetCollisionEnabled` (`self.CapsuleComponent`) "NoCollision")))

(event `self.ReceiveBeginPlay`
  (`ActorComponent.Activate` (`self.CharacterMovement`) false))

(event `self.ReceiveTick`
  (params (DeltaSeconds :type "Float (single-precision)"))
  (`self.AddMovementInput` (0.05 0.0 0.0)))

(fn `UserConstructionScript`)