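; Side-scrolling enemy character that chases the player along the X axis and deals contact damage.
; A sight collider toggles the chase; Tick feeds movement input toward the player and flips yaw from X velocity.
; Tick also polls attack-collider overlaps, applying damage through a DoOnce that resets after a delay while alive.
; Incoming damage lowers health; exactly zero disables movement and collision, then destroys the actor after a short delay.
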(event `self.ReceiveAnyDamage`
  (params (Damage :type "Float (single-precision)") (DamageType :type "DamageType Object Reference") (InstigatedBy :type "Controller Object Reference") (DamageCauser :type "Actor Object Reference"))
  (bind _output_get (set `self.Health` (- (`self.Health`) Damage)))
  (if (== _output_get 0.0)
    (set `self.isDead` true)
    (`ActorComponent.SetActive` (`self.CharacterMovement`) false false)
    (`PrimitiveComponent.SetCollisionEnabled` (`self.CapsuleComponent`) "NoCollision")
    (`KismetSystemLibrary.Delay` 0.5)
    (`self.K2_DestroyActor`)))

(event `self.Attack_Collision.OnComponentBeginOverlap`
  (params (OverlappedComponent :type "PrimitiveComponent Object Reference") (OtherActor :type "Actor Object Reference") (OtherComp :type "PrimitiveComponent Object Reference") (OtherBodyIndex :type Integer) (bFromSweep :type Boolean) (SweepResult :type "HitResult Structure (by ref)"))
  (if (== OtherActor null)
    _))

(event `self.ReceiveTick`
  (params (DeltaSeconds :type "Float (single-precision)"))
  (bind _returnvalue (`GameplayStatics.GetPlayerCharacter` 0))
  (bind _returnvalue_x (`KismetMathLibrary.BreakVector` (`SceneComponent.K2_GetComponentLocation` (`self.CapsuleComponent`))))
  (`|ExecutionSequence`
    (:`then_0`
      (`self.EnemyRotation`)
      (if (`self.IsSeeingPlayer`)
        (bind _asplayer (cast `/Game/Reordered/Blueprints/Player/Player` (`GameplayStatics.GetPlayerCharacter` 0)))
        (bind _returnvalue_x_2 (`KismetMathLibrary.BreakVector` (`SceneComponent.K2_GetComponentLocation` (`Character.CapsuleComponent` _asplayer))))
        (bind _returnvalue_2 (- _returnvalue_x_2 _returnvalue_x))
        (if (>= _returnvalue_2 0.0)
          (set `self.isMovingRight` true)
          (else
            (set `self.isMovingRight` false)))
        (`self.AddMovementInput` (0.1 0.0 0.0) (`KismetMathLibrary.SignOfFloat` _returnvalue_2))))
    (:`then_1`
      (for _array_element (`PrimitiveComponent.GetOverlappingActors` (`self.Attack_Collision`) "/Game/Reordered/Blueprints/Player/Player.Player_C")
        (if (== _array_element _returnvalue)
          (`/Engine/EditorBlueprintResources/StandardMacros.DoOnce` false :!label _label
            (:`Completed`
              (`GameplayStatics.ApplyDamage` _returnvalue 1.0)
              (`KismetSystemLibrary.Delay` 1.0)
              (if (not (`self.isDead`))
                (goto _label :!via `Reset`)))))))))

(event `self.Sight_Collider.OnComponentBeginOverlap`
  (params (OverlappedComponent :type "PrimitiveComponent Object Reference") (OtherActor :type "Actor Object Reference") (OtherComp :type "PrimitiveComponent Object Reference") (OtherBodyIndex :type Integer) (bFromSweep :type Boolean) (SweepResult :type "HitResult Structure (by ref)"))
  (cast `/Game/Reordered/Blueprints/Player/Player` OtherActor)
  (set `self.IsSeeingPlayer` true))

(event `self.Sight_Collider.OnComponentEndOverlap`
  (params (OverlappedComponent :type "PrimitiveComponent Object Reference") (OtherActor :type "Actor Object Reference") (OtherComp :type "PrimitiveComponent Object Reference") (OtherBodyIndex :type Integer))
  (cast `/Game/Reordered/Blueprints/Player/Player` OtherActor)
  (set `self.IsSeeingPlayer` false))

(fn `EnemyRotation`
  (bind _velocity_x (`KismetMathLibrary.BreakVector` (`MovementComponent.Velocity` (`self.CharacterMovement`))))
  (`/Engine/EditorBlueprintResources/StandardMacros.CompareFloat` _velocity_x
    (:`>`
      (`self.K2_SetActorRotation` (`KismetMathLibrary.MakeRotator` 0.0)))
    (:`<`
      (`self.K2_SetActorRotation` (`KismetMathLibrary.MakeRotator` 0.0 0.0 180.0)))))

(fn `UserConstructionScript`)